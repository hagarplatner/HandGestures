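; XR hand Blueprint that records, deletes and recognizes named hand gestures from bone poses.
; Recording stores every bone's component-space location under a unique name in a BP_SaveGameGestures save slot, loaded on BeginPlay.
; A looping timer, used instead of Tick, picks the first saved gesture with all bones within a distance threshold.
; OnGestureRecognized fires only when that match differs from the current gesture.
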(event Custom|DetectGesture
  ;[0.3451 0.4235 1] Delete Gesture
  (bind (_result _gesture) (CallFunction|GetCurrentGesture))
  (if _result
    (if (not (CallFunction|EqualGestures _gesture (Variables|Default|GetCurrentGesture)))
      (bind _output_get (Variables|Default|SetCurrentGesture _gesture))
      (Default|CallOnGestureRecognized (.GestureName (Utilities|Struct|BreakS_HandGestures _output_get))))))

(event EventBeginPlay
  ;[0.3451 0.4235 1] Load Gestures
  (Variables|Default|SetGestures (Variables|/Game/Assets/HandGestures/BP_SaveGameGestures.BP_SaveGameGestures_C|GetGestures (CallFunction|LoadGestures)))
  (Utilities|Time|SetTimerbyEvent (delegate Custom|DetectGesture) (Variables|Default|GetRefreshRate) true))

(event EventTick
  (params (DeltaSeconds :type Float%20%28single-precision%29)))

(fn LoadGestures
  ;[0.3451 0.4235 1] Check if save game file exist
  (bind _returnvalue (SaveGame|DoesSaveGameExist (Variables|Default|GetGestureNameSlot)))
  (if _returnvalue
    ;[0.3451 0.4235 1] Load save game and return it
    (bind _returnvalue_2 (SaveGame|LoadGamefromSlot (Variables|Default|GetGestureNameSlot)))
    (bind _asbp_save_game_gestures (Utilities|Casting|CastToBP_SaveGameGestures _returnvalue_2))
    (return _asbp_save_game_gestures)
    (else
      ;[0.3451 0.4235 1] create a save game if it doesn't exist and return it
      (bind _returnvalue_3 (SaveGame|CreateSaveGameObject "/Game/Assets/HandGestures/BP_SaveGameGestures.BP_SaveGameGestures_C"))
      (return _returnvalue_3))))

(fn RecordGesture
  (params (GestureName :type String))
  ;[0.3451 0.4235 1] Check if gesture exist already
  (bind _output_get (LocalVariables|SetGestureSaveGame (CallFunction|LoadGestures)))
  (bind _return (CallFunction|DoesGestureExist? _output_get GestureName))
  (if (not _return)
    ;[0.3451 0.4235 1] if gesture does not exist save bone locations
    (for _index (range 0 (- (Class|SkinnedMeshComponent|GetNumBones) 1))
      (bind _returnvalue (Class|PoseableMeshComponent|GetBoneLocationbyName (Class|SkinnedMeshComponent|GetBoneName _index) "ComponentSpace"))
      (Utilities|Array|Add (LocalVariables|GetBoneLocations) _returnvalue))
    ;[0.3451 0.4235 1] When finished add to gestures array and save game to slot
    (Utilities|Array|Add (Variables|/Game/Assets/HandGestures/BP_SaveGameGestures.BP_SaveGameGestures_C|GetGestures (LocalVariables|GetGestureSaveGame)) (Utilities|Struct|MakeS_HandGestures GestureName (LocalVariables|GetBoneLocations)))
    (SaveGame|SaveGametoSlot (LocalVariables|GetGestureSaveGame) (Variables|Default|GetGestureNameSlot))))

(fn DoesGestureExist?
  (params (SaveGameGesture :type BP%20Save%20Game%20Gestures%20Object%20Reference) (GestureName :type String))
  ;[0.3451 0.4235 1] go through all gestures in array
  (for _array_element (Variables|/Game/Assets/HandGestures/BP_SaveGameGestures.BP_SaveGameGestures_C|GetGestures SaveGameGesture)
    ;[0.3451 0.4235 1] if same gesture return true
    (if (Utilities|Enum|Equal(Enum) (.GestureName (Utilities|Struct|BreakS_HandGestures _array_element)) GestureName)
      (return true)))
  ;[0.3451 0.4235 1] if different gesture return false
  (return false))

(fn DeleteGesture
  (params (GestureName :type String))
  ;[0.3451 0.4235 1] go through all gestures
  (bind _output_get (LocalVariables|SetGestureSaveGame (CallFunction|LoadGestures)))
  (for (_array_element _array_index) (Variables|/Game/Assets/HandGestures/BP_SaveGameGestures.BP_SaveGameGestures_C|GetGestures _output_get)
    ;[0.3451 0.4235 1] if found gesture save index
    (if (Utilities|Enum|Equal(Enum) (.GestureName (Utilities|Struct|BreakS_HandGestures _array_element)) GestureName)
      (LocalVariables|SetIndex _array_index)))
  ;[0.3451 0.4235 1] when finished remove gesture with index and save game to slot
  (Utilities|Array|RemoveIndex (Variables|/Game/Assets/HandGestures/BP_SaveGameGestures.BP_SaveGameGestures_C|GetGestures (LocalVariables|GetGestureSaveGame)) (LocalVariables|GetIndex))
  (SaveGame|SaveGametoSlot (LocalVariables|GetGestureSaveGame) (Variables|Default|GetGestureNameSlot)))

(fn GetCurrentGesture
  ;[0.3451 0.4235 1] go through all gestures
  (for _array_element (Variables|Default|GetGestures)
    ;[0.3451 0.4235 1] find bone location
    (for (_array_element_2 _array_index) (.BoneLocations (Utilities|Struct|BreakS_HandGestures _array_element))
      (bind _returnvalue (Class|PoseableMeshComponent|GetBoneLocationbyName (Class|SkinnedMeshComponent|GetBoneName _array_index) "ComponentSpace"))
      ;[0.3451 0.4235 1] Debug - print length
      (if (Variables|Default|GetDebug)
        (Development|PrintString (Utilities|String|ToString(Float) (Math|Float|Absolute(Float) (Math|Vector|VectorLength (- _returnvalue _array_element_2))))))
      ;[0.3451 0.4235 1] check if length bigger then treshold
      (if (> (Math|Float|Absolute(Float) (Math|Vector|VectorLength (- _returnvalue _array_element_2))) (Variables|Default|GetTreshold))
        (LocalVariables|SetBvalidGesture? false)))
    ;[0.3451 0.4235 1] check if found gesture
    (if (LocalVariables|GetBvalidGesture?)
      ;[0.3451 0.4235 1] if true loop ends and send the gesture
      (return (LocalVariables|GetBvalidGesture?) _array_element)
      (else
        ;[0.3451 0.4235 1] if false make it true and continue loop
        (LocalVariables|SetBvalidGesture? true))))
  ;[0.3451 0.4235 1] if we got here meaning we didn't find gesture
  (return false ""))

(fn EqualGestures
  (params (A :type S%20Hand%20Gestures%20Structure) (B :type S%20Hand%20Gestures%20Structure))
  (bind (_gesturename _bonelocations) (Utilities|Struct|BreakS_HandGestures A))
  (bind (_gesturename_2 _bonelocations_2) (Utilities|Struct|BreakS_HandGestures B))
  (return (and (Utilities|Enum|Equal(Enum) _gesturename _gesturename_2) (Utilities|Array|Identical _bonelocations _bonelocations_2))))